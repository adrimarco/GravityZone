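; Gravity controller that handles look and orientation for the player's BP_SoldierCharacter under a changeable gravity direction.
; IA_Look input accumulates yaw and clamped pitch, which Tick composes with the movement component's WorldToGravityTransform quaternion to rotate the body by yaw and the first-person camera by both.
; ChangeGravity turns the stored gravity vector a quarter turn around world X and applies it to character movement, with no caller in this graph.
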(event `self.ReceiveBeginPlay`
  (bind _asbp_soldier_character (cast `/Game/Blueprints/Character/BP_SoldierCharacter` (`GameplayStatics.GetPlayerCharacter` 0)))
  (bind _output_get (set `self.PlayerCharacter` _asbp_soldier_character)))

(event `self.ReceiveTick`
  (params (DeltaSeconds :type "Float (single-precision)"))
  (`self.UpdateActorRotation`))

(event `EnhancedInput|/Game/Input/Actions/IA_Look`
  (params (ActionValue :type "Vector2D Structure") (ElapsedSeconds :type "Float (double-precision)") (TriggeredSeconds :type "Float (double-precision)") (InputAction :type "InputAction Object Reference" :default "/Game/Input/Actions/IA_Look.IA_Look"))
  (:`Triggered`
    (`self.Look` ActionValue)))

(fn `ChangeGravity`
  (bind _output_get (set `self.GravityDir` (`KismetMathLibrary.RotateAngleAxis` (`self.GravityDir`) 90.0 (1.0 0.0 0.0))))
  (`CharacterMovementComponent.SetGravityDirection` (`Character.CharacterMovement` (`self.PlayerCharacter`)) _output_get))

(fn `Look`
  (params (Value :type "Vector2D Structure"))
  (bind (_x _y) (`KismetMathLibrary.BreakVector2D` Value))
  (set `self.Yaw` (`KismetMathLibrary.ClampAxis` (+ (`self.Yaw`) _x)))
  (set `self.Pitch` (`KismetMathLibrary.FClamp` (- (`self.Pitch`) _y) -80.0 80.0)))

(fn `UpdateActorRotation`
  (bind _playercharacter (`self.PlayerCharacter`))
  (bind _worldtogravitytransform (`CharacterMovementComponent.WorldToGravityTransform` (`Character.CharacterMovement` (`self.PlayerCharacter`))))
  (`Actor.K2_SetActorRotation` _playercharacter (`KismetMathLibrary.Quat_Rotator` (* _worldtogravitytransform (`KismetMathLibrary.Conv_RotatorToQuaternion` (`KismetMathLibrary.MakeRotator` 0.0 0.0 (`self.Yaw`))))) false)
  (`SceneComponent.K2_SetWorldRotation` (`SoldierCharacter.FPCamera` _playercharacter) (`KismetMathLibrary.Quat_Rotator` (* _worldtogravitytransform (`KismetMathLibrary.Conv_RotatorToQuaternion` (`KismetMathLibrary.MakeRotator` 0.0 (`self.Pitch`) (`self.Yaw`))))) false false))