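; BP_SoldierCharacter is a soldier character that arms itself and shows a HUD when play begins.
; On BeginPlay it adds two weapons, an AK and a Glock, through AddNewWeapon.
; If controlled by the first player controller, it creates a BP_SoldierHUD widget, adds it to the viewport and binds it to itself.
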(event `self.ReceiveBeginPlay`
  (bind _returnvalue (`self.GetController`))
  (`self.AddNewWeapon` (enumliteral `EWeaponId` "AK"))
  (`self.AddNewWeapon` (enumliteral `EWeaponId` "Glock"))
  (if (== (`GameplayStatics.GetPlayerController` 0) _returnvalue)
    (bind _returnvalue_2 (`|CreateWidget` "/Game/UI/BP_SoldierHUD.BP_SoldierHUD_C" (cast `PlayerController` _returnvalue :!pure true)))
    (`UserWidget.AddToViewport` _returnvalue_2 0)
    (`SoldierHUD.BindToSoldierCharacter` _returnvalue_2 self)))

(fn `UserConstructionScript`)